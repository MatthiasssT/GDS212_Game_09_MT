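; BP_Keg is an interactable keg that refills the player's drink.
; Look-at events toggle custom depth on the keg mesh, likely for a highlight, and show or hide an interact prompt widget.
; Interact prints a debug string and sends a RefillDrink message to the object passed in, leaving the refill logic to that target.
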(event `/Game/_Main/Interfaces/BPI_Interact.NotLookingAt`
  (`self.Player Stopped Looking At`))

(event `/Game/_Main/Interfaces/BPI_Interact.LookingAt`
  (`self.Player Looking at`))

(event `Player Looking at`
  (`PrimitiveComponent.SetRenderCustomDepth` (`self.KegMesh`) true)
  (`SceneComponent.SetVisibility` (`self.WBP_Interact`) true false))

(event `Player Stopped Looking At`
  (`PrimitiveComponent.SetRenderCustomDepth` (`self.KegMesh`) false)
  (`SceneComponent.SetVisibility` (`self.WBP_Interact`) false false))

(event `/Game/_Main/Interfaces/BPI_Interact.Interact`
  (params (`Object to refill` :type "Actor Object Reference"))
  ;[1 1 1] Call refil on drink as target
  (`KismetSystemLibrary.PrintString` "called refill drink")
  (message `/Game/_Main/Interfaces/BPI_Interact.RefillDrink` `Object to refill`))

(fn `UserConstructionScript`)