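; BP_Customer is a customer actor that the player can start a dialogue with.
; Look-at events show and hide its TalkWidget as the player looks at or away from it.
; The speaking event stores the player's speaker component and, if valid, starts dialogue owned by the customer's BPCSpeakerComponent with both speakers as participants.
; Debug prints trace the attempt, including an invalid player reference.
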(event `Player Is looking at`
  ;[1 1 1] Player looking at logic
  (`SceneComponent.SetVisibility` (`self.TalkWidget`) true false))

(event `Player is not looking at`
  ;[1 1 1] Player looking at logic
  (`SceneComponent.SetVisibility` (`self.TalkWidget`) false false))

(event `Player Speaking with`
  (params (`Player BPC speaker ref` :type "/DialogueTree/Blueprints/SpeakerComponents/BPC_SpeakerComponent Object Reference"))
  (bind _bpc_speakercomponent (`self.BPC_SpeakerComponent`))
  (set `self.Player Speaker Ref` `Player BPC speaker ref`)
  (`KismetSystemLibrary.PrintString` "Player is speaking with customer")
  (bind _player_speaker_ref (`self.Player Speaker Ref`)
    (:`then`
      (`KismetSystemLibrary.PrintString` "Dialogue entered" true true (struct :`R` 1.0 :`G` 0.989155 :`A` 1.0))
      (`DialogueSpeakerComponent.StartOwnedDialogue` _bpc_speakercomponent (`|MakeArray` _bpc_speakercomponent _player_speaker_ref :!type "DialogueSpeakerComponent Object Reference")))
    (:`else`
      (`KismetSystemLibrary.PrintString` "boooo" true true (struct :`R` 1.0 :`B` 0.071863 :`A` 1.0)))))

(fn `UserConstructionScript`)