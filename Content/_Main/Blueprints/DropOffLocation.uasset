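; DropOffLocation is a work-in-progress actor meant to track beers placed on a table or counter.
; Every Tick it scans the BeersOnTable array for a full drink and prints debug messages, with the full-beer message gated on a separate ABeerIsFull flag.
; A custom event sets ABeerIsOnTable when a beer is added.
; The Trigger overlap events are empty, and the tag-based add/remove logic from an abandoned attempt is disconnected.
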(event `self.ReceiveBeginPlay`)

(event `self.ReceiveTick`
  (params (DeltaSeconds :type "Float (single-precision)"))
  (if (< (`KismetArrayLibrary.Array_Length` (`self.Beers on table`)) 0)
    _
    (else
      _))
  (`self.There is a beer on the table`)
  (`KismetSystemLibrary.PrintString` "there is a beer on the table"))

(event `Beer has been added`
  (set `self.A beer is on table?` true))

(event `Beer has been removed`)

(event `There is a beer on the table`
  (for (_array_element _array_index) (`self.Beers on table`)
    (if (`/Game/_Main/Blueprints/BP_Beer.Drink is full?` _array_element)
      (break)))
  (if (`self.A Beer is full?`)
    (`KismetSystemLibrary.PrintString` "full beer is on the table" true true (struct :`G` 1.0 :`B` 0.159937 :`A` 1.0))))

(event `self.trigger.OnComponentBeginOverlap`
  (params (OverlappedComponent :type "PrimitiveComponent Object Reference") (OtherActor :type "Actor Object Reference") (OtherComp :type "PrimitiveComponent Object Reference") (OtherBodyIndex :type Integer) (bFromSweep :type Boolean) (SweepResult :type "HitResult Structure (by ref)"))
  ;[1 1 1] First attempt did not work
  ;;[1 1 1] event trigger
)

(event `self.trigger.OnComponentEndOverlap`
  (params (OverlappedComponent :type "PrimitiveComponent Object Reference") (OtherActor :type "Actor Object Reference") (OtherComp :type "PrimitiveComponent Object Reference") (OtherBodyIndex :type Integer))
  ;[1 1 1] First attempt did not work
  ;;[1 1 1] event trigger
)

(fn `UserConstructionScript`)