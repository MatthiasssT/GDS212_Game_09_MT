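; Radio system Blueprint that plays an endless shuffle of non-spatial 2D songs from a song list, starting on BeginPlay.
; ChangeSong fades out any valid current audio, spawns the next song, waits for its duration with a Delay, then calls itself again.
; SelectNewSong picks at random and retries until the pick differs from the current song, so a one-song list would loop endlessly after the first play.
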(event `self.ReceiveBeginPlay`
  (`self.ChangeSong`))

(event `ChangeSong`
  (`self.FadeOut`)
  (if true
    (set `self.CurrentSong` (`self.SelectNewSong`)))
  (bind _returnvalue (`GameplayStatics.SpawnSound2D` (`self.CurrentSong`) 0.75 1.0 0.0 null))
  (set `self.CurrentSongRef` _returnvalue)
  (`KismetSystemLibrary.Delay` (`SoundBase.Duration` (`self.CurrentSong`)))
  (`self.ChangeSong`))

(fn `FadeOut`
  (returns (`Faded Out?` :type Boolean))
  (bind _currentsongref (`self.CurrentSongRef`)
    (:`then`
      (`AudioComponent.FadeOut` _currentsongref 1.0 0.0 "Linear")
      (return true))
    (:`else`
      (return false))))

(fn `SelectNewSong`
  (returns (SelectedSong :type "SoundBase Object Reference"))
  (locals (ProvSong :type "SoundBase Object Reference"))
  (bind _songlist (`self.Songlist`))
  (set `local.ProvSong` (`|GetArrayItem` _songlist (`KismetMathLibrary.RandomIntegerInRange` 0 (`KismetArrayLibrary.Array_LastIndex` _songlist))) :!label _label)
  (if (== (`self.CurrentSong`) (`local.ProvSong`))
    (goto _label)
    (else
      (return (`local.ProvSong`)))))