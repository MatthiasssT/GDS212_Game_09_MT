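; BP_DropOffLocation is a table drop-off point that tracks beers and hands a full one to a customer.
; An event scans the BeersOnTable array, storing a full beer's reference and setting a flag, which each later element can overwrite.
; Giving a beer destroys the stored actor after a short delay, then spawns a new BP_Beer at its transform.
; Trigger overlaps only print debug messages for Beer-tagged actors, leaving the array untouched.
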(event `self.ReceiveBeginPlay`)

(event `self.ReceiveTick`
  (params (DeltaSeconds :type "Float (single-precision)")))

(event `There is a beer on the table`
  (bind _beers_on_table (`self.Beers on table`))
  ;[0.05098 0.05098 0.05098] Beer on table logic
  ;;[1 1 1] Called when a beer is on table. adds item to the array and gets reference to if a beer is full on the table and its index
  (for (_array_element _array_index) _beers_on_table
    (if (`/Game/_Main/Blueprints/BP_Beer.Drink is full?` _array_element)
      (`KismetSystemLibrary.PrintString` "full beer is on the table" true true (struct :`G` 1.0 :`B` 0.159937 :`A` 1.0))
      (bind _output (`|GetArrayItem` _beers_on_table _array_index))
      (if (== _array_element _output)
        (set `self.Beer that is on the table` _output)
        (`KismetSystemLibrary.PrintText` (`|FormatText` "beer that is full is {ArrayIndex} in the array" _array_index) true true (struct :`R` 0.120343 :`G` 1.0 :`A` 1.0))
        (set `self.A Beer is full?` true)
        (else
          (`KismetSystemLibrary.PrintString` "cant get ref to index of beer" true true (struct :`R` 1.0 :`G` 0.025198 :`A` 1.0))))
      (else
        (`KismetSystemLibrary.PrintString` "all beers empty" true true (struct :`R` 1.0 :`G` 0.040385 :`A` 1.0))
        (set `self.A Beer is full?` false)))))

(event `self.trigger.OnComponentBeginOverlap`
  (params (OverlappedComponent :type "PrimitiveComponent Object Reference") (OtherActor :type "Actor Object Reference") (OtherComp :type "PrimitiveComponent Object Reference") (OtherBodyIndex :type Integer) (bFromSweep :type Boolean) (SweepResult :type "HitResult Structure (by ref)"))
  ;[0.05098 0.05098 0.05098] Beer on table logic
  ;;[1 1 1] event trigger
  (if (`self.ActorHasTag` OtherActor "Beer")
    (`KismetSystemLibrary.PrintString` "beer on the table" true true (struct :`R` 1.0 :`G` 0.671306 :`A` 1.0))))

(event `self.trigger.OnComponentEndOverlap`
  (params (OverlappedComponent :type "PrimitiveComponent Object Reference") (OtherActor :type "Actor Object Reference") (OtherComp :type "PrimitiveComponent Object Reference") (OtherBodyIndex :type Integer))
  ;[0.05098 0.05098 0.05098] Beer on table logic
  ;;[1 1 1] event trigger
  (if (`self.ActorHasTag` OtherActor "Beer")
    (`KismetSystemLibrary.PrintString` "beer removed from the table" true true (struct :`R` 1.0 :`G` 0.671306 :`A` 1.0))))

(event `Give Full Beer to Customer`
  ;[0.05098 0.05098 0.05098] Beer on table logic
  ;;[1 1 1] Beer drink method (give to customer)
  (if (`self.A Beer is full?`)
    (bind _beer_that_is_on_the_table (`self.Beer that is on the table`)
      (:`then`
        (set `self.Full Beer Location` (`self.GetTransform` _beer_that_is_on_the_table))
        (`KismetSystemLibrary.Delay` 0.5)
        (`self.K2_DestroyActor` _beer_that_is_on_the_table)
        (`KismetSystemLibrary.Delay` 0.5)
        (`|SpawnActorFromClass` "/Game/_Main/Blueprints/BP_Beer.BP_Beer_C" (`self.Full Beer Location`) "AlwaysSpawn" "OverrideRootScale" null null)
        (set `self.Full Beer Location` (struct)))
      (:`else`))
    (else
      (`KismetSystemLibrary.PrintString` "sorry let me get you a full cup"))))

(fn `UserConstructionScript`)